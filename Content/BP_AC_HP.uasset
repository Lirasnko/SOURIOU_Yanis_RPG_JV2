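; BP_AC_HP is a health component, by its name an Actor Component, that tracks HP and destroys an actor when it runs out.
; HPModification adds positive quantities up to HPMax; otherwise it compares HP with a value derived from Quantity.
; If HP is higher, it subtracts the signed Quantity, so negative input raises HP without clamping.
; Otherwise it zeroes HP and calls Death, which destroys the referenced Actor.
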(event EventBeginPlay)

(event EventTick
  (params (DeltaSeconds :type Float%20%28single-precision%29)))

(fn HPModification
  (params (Quantity :type Integer))
  (bind _hpmax (Variables|Default|GetHPMax))
  (if (> Quantity 0)
    (if (> (- _hpmax (Variables|Default|GetHP)) Quantity)
      (Variables|Default|SetHP (+ (Variables|Default|GetHP) Quantity))
      (else
        (Variables|Default|SetHP _hpmax)))
    (else
      (bind _result (Utilities|NegateInt Quantity)
        (:%20%20
          (if (> (Variables|Default|GetHP) _result)
            (Variables|Default|SetHP (- (Variables|Default|GetHP) Quantity))
            (else
              (Variables|Default|SetHP 0)
              (CallFunction|Death))))))))

(fn Death
  (Actor|DestroyActor (Variables|Default|GetActor)))
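; BP_IA_Master is an AI actor, named as a master class, that shows damage feedback and dies at zero HP.
; BeginPlay registers the actor with its BPACHP health component.
; TakeDamage spawns a BP_Damage actor slightly above it, passes in the damage value, then destroys itself if the component's HP is depleted.
; The event does not subtract HP itself.
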(event Custom|TakeDamage
  (params (damage :type Integer))
  (bind _returnvalue (Transformation|GetActorLocation))
  (bind _returnvalue_2 (Game|SpawnActorfromClass "/Game/Blueprints/BP_Damage.BP_Damage_C" (Math|Transform|MakeTransform (Math|Vector|MakeVector (.x _returnvalue) (.y _returnvalue) (+ (.z _returnvalue) 5e+01)) "0, 0, 0" "1.000000,1.000000,1.000000") "Undefined" "MultiplyWithRoot" 0 0))
  (Default|SetValue _returnvalue_2 damage)
  (if (<= (Variables|/Game/Blueprints/Component/BP_AC_HP.BP_AC_HP_C|GetHP (Variables|Default|GetBP_AC_HP)) 0)
    (Actor|DestroyActor)))

(event EventBeginPlay
  (Variables|/Game/Blueprints/Component/BP_AC_HP.BP_AC_HP_C|SetActor (Variables|Default|GetBP_AC_HP) self))

(event Collision|EventActorBeginOverlap
  (params (OtherActor :type Actor%20Object%20Reference)))

(event EventTick
  (params (DeltaSeconds :type Float%20%28single-precision%29)))

(fn ConstructionScript)
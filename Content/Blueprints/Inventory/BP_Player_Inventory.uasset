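; BP_Player_Inventory is a character preview actor that mirrors the player's equipped gear, apparently for the inventory screen.
; Every Tick it applies the top-down controller's InventoryPlayer rotation and loops over its Equipment map keys.
; Weapon data assets fill one of two meshes, chosen by comparing their icon to the sword sprite.
; Armor assets set static helmet or skeletal body-part meshes by Type; nothing clears unequipped slots.
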(event EventBeginPlay)

(event Collision|EventActorBeginOverlap
  (params (OtherActor :type Actor%20Object%20Reference)))

(event EventTick
  (params (DeltaSeconds :type Float%20%28single-precision%29))
  (bind _playercontroler (CallFunction|GetTopDownController))
  (Transformation|SetRelativeRotation (Variables|Default|GetPlayer) (Variables|/Game/TopDown/Blueprints/BP_TopDownController.BP_TopDownController_C|GetInventoryPlayer _playercontroler) false false)
  (bind _keypin (Utilities|Map|ForEachLoop(Map) (Variables|/Game/TopDown/Blueprints/BP_TopDownController.BP_TopDownController_C|GetEquipment _playercontroler))
    (:then
      (bind _asbp_pda_weapons_items (Utilities|Casting|CastToBP_PDA_Weapons_Items _keypin)
        (:then
          (if (== (Variables|/Game/Blueprints/Data/BP_PDA_Items.BP_PDA_Items_C|GetValueIcon _asbp_pda_weapons_items) "/Game/Textures/Sprites/T_Sword_Sprite.T_Sword_Sprite")
            (Components|StaticMesh|SetStaticMesh (Variables|Default|GetWeapon1) (Variables|/Game/Blueprints/Data/BP_PDA_Items.BP_PDA_Items_C|GetMesh _asbp_pda_weapons_items))
            (else
              (Components|StaticMesh|SetStaticMesh (Variables|Default|GetWeapon2) (Variables|/Game/Blueprints/Data/BP_PDA_Items.BP_PDA_Items_C|GetMesh _asbp_pda_weapons_items)))))
        (:CastFailed
          (bind _asbp_pda_armors_items (Utilities|Casting|CastToBP_PDA_Armors_Items _keypin))
          (switch Utilities|FlowControl|Switch|SwitchonE_Armor (Variables|/Game/Blueprints/Data/BP_PDA_Armors_Items.BP_PDA_Armors_Items_C|GetType _asbp_pda_armors_items)
            (:NewEnumerator0
              (Components|StaticMesh|SetStaticMesh (Variables|Default|GetHelmet) (Variables|/Game/Blueprints/Data/BP_PDA_Items.BP_PDA_Items_C|GetMesh _asbp_pda_armors_items)))
            (:NewEnumerator1
              (Components|SkeletalMesh|SetSkeletalMeshAsset (Variables|Default|GetChestplate) (Variables|/Game/Blueprints/Data/BP_PDA_Armors_Items.BP_PDA_Armors_Items_C|GetSkeletalMesh _asbp_pda_armors_items)))
            (:NewEnumerator2
              (Components|SkeletalMesh|SetSkeletalMeshAsset (Variables|Default|GetArm) (Variables|/Game/Blueprints/Data/BP_PDA_Armors_Items.BP_PDA_Armors_Items_C|GetSkeletalMesh _asbp_pda_armors_items)))
            (:NewEnumerator3
              (Components|SkeletalMesh|SetSkeletalMeshAsset (Variables|Default|GetLegging) (Variables|/Game/Blueprints/Data/BP_PDA_Armors_Items.BP_PDA_Armors_Items_C|GetSkeletalMesh _asbp_pda_armors_items)))
            (:NewEnumerator4
              (Components|SkeletalMesh|SetSkeletalMeshAsset (Variables|Default|GetBoot) (Variables|/Game/Blueprints/Data/BP_PDA_Armors_Items.BP_PDA_Armors_Items_C|GetSkeletalMesh _asbp_pda_armors_items)))))))))

(fn ConstructionScript)
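; Actor that displays a 3D mesh of the currently selected inventory or shop item.
; Each Tick it polls the game widget's infinite inventory, inventory and shop, in that priority, clearing the mesh when none has a current item.
; ChangeCurrentItem applies the item's mesh, elevation, angle and size, adding a small yaw step per update to spin it.
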(event EventBeginPlay)

(event Collision|EventActorBeginOverlap
  (params (OtherActor :type Actor%20Object%20Reference)))

(event EventTick
  (params (DeltaSeconds :type Float%20%28single-precision%29))
  (bind _playercontroler (CallFunction|GetTopDownController))
  (bind _widgetgame (Variables|/Game/TopDown/Blueprints/BP_TopDownController.BP_TopDownController_C|GetWidgetGame _playercontroler))
  (bind _widget_infiniteinventory (Variables|/Game/Widget/WBP_Game.WBP_Game_C|GetWidget_InfiniteInventory _widgetgame))
  (bind _widget_inventory (Variables|/Game/Widget/WBP_Game.WBP_Game_C|GetWidget_Inventory _widgetgame))
  (bind _widget_shop (Variables|/Game/Widget/WBP_Game.WBP_Game_C|GetWidget_Shop _widgetgame))
  (bind _currentitem (Variables|/Game/Widget/WBP_InfiniteInventory.WBP_InfiniteInventory_C|GetCurrentItem _widget_infiniteinventory))
  (bind _currentitem_2 (Variables|/Game/Widget/WBP_Inventory.WBP_Inventory_C|GetCurrentItem _widget_inventory))
  (bind _currentitem_3 (Variables|/Game/Widget/WBP_Shop.WBP_Shop_C|GetCurrentItem _widget_shop))
  (if (Utilities|IsValid _currentitem)
    (CallFunction|ChangeCurrentItem _currentitem)
    (elif (Utilities|IsValid _currentitem_2)
      (CallFunction|ChangeCurrentItem _currentitem_2)
      (elif (Utilities|IsValid _currentitem_3)
        (CallFunction|ChangeCurrentItem _currentitem_3)
        (else
          (Components|StaticMesh|SetStaticMesh (Variables|Default|GetMesh) 0))))))

(fn ConstructionScript)

(fn ChangeCurrentItem
  (params (Item :type BP%20PDA%20Items%20Object%20Reference))
  (bind _mesh (Variables|/Game/Blueprints/Data/BP_PDA_Items.BP_PDA_Items_C|GetMesh Item))
  (bind _mesh_2 (Variables|Default|GetMesh))
  (bind _size (Variables|/Game/Blueprints/Data/BP_PDA_Items.BP_PDA_Items_C|GetSize Item))
  (bind _mesh_3 (Variables|Default|GetMesh))
  (if (!= _mesh_3 _mesh)
    (Components|StaticMesh|SetStaticMesh _mesh_3 _mesh)
    (Transformation|SetRelativeTransform _mesh_2 (Math|Transform|MakeTransform (Math|Vector|MakeVector 0.0 0.0 (Math|Conversions|ToFloat(Integer) (Variables|/Game/Blueprints/Data/BP_PDA_Items.BP_PDA_Items_C|GetElevation Item))) (Math|Rotator|CombineRotators (Math|Rotator|MakeRotator (Variables|/Game/Blueprints/Data/BP_PDA_Items.BP_PDA_Items_C|GetAngle Item) 0.0 (.yaw (Variables|/Script/Engine.SceneComponent|GetRelativeRotation _mesh_2))) "0.000000,2.000000,0.000000") (Math|Vector|MakeVector _size _size _size)) false false)))
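; Throwable bomb actor that explodes on its first impact, damaging nearby AI characters and breakable rocks.
; A sphere collision hit spawns the Niagara explosion, hides the mesh, flags damage and destroys the actor after a short delay.
; Tick consumes that flag once, scanning a second sphere's overlaps.
; AI characters take random damage through their HP component and are launched outward and upward, while rocks receive a fixed HP change.
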(event OnComponentHit(Sphere)
  (params (HitComponent :type Primitive%20Component%20Object%20Reference) (OtherActor :type Actor%20Object%20Reference) (OtherComp :type Primitive%20Component%20Object%20Reference) (NormalImpulse :type Vector :default "0, 0, 0") (Hit :type Hit%20Result%20Structure%20%28by%20ref%29))
  (if (Variables|Default|GetdoExplose)
    (Variables|Default|SetdoExplose false)
    (Niagara|SpawnSystematLocation "/Game/Effect/NS_Explosion.NS_Explosion" (.location Hit))
    (Variables|Default|SetdoDamage true)
    (Rendering|SetVisibility (Variables|Character|GetMesh) false false)
    (Utilities|FlowControl|Delay 0.2)
    (Actor|DestroyActor)))

(event EventBeginPlay
  (|CallParentFunction) ; This node is disabled and will not be called.\nDrag off pins to build functionality.
)

(event Collision|EventActorBeginOverlap
  (params (OtherActor :type Actor%20Object%20Reference))
  (|CallParentFunction OtherActor) ; This node is disabled and will not be called.\nDrag off pins to build functionality.
)

(event EventTick
  (params (DeltaSeconds :type Float%20%28single-precision%29))
  (|CallParentFunction DeltaSeconds)
  (if (Variables|Default|GetdoDamage)
    (Variables|Default|SetdoDamage false)
    (for _array_element (Collision|GetOverlappingActors (Variables|Default|GetSphere_0) 0 :!class /Script/Engine.PrimitiveComponent)
      (bind _asbp_ia_master (Utilities|Casting|CastToBP_IA_Master _array_element)
        (:then
          (bind _output_get (Variables|Default|SetDamage (Math|Random|RandomIntegerinRange (Variables|Default|GetMinDamage) (Variables|Default|GetMaxDamage))))
          (Default|HPModification (Variables|/Game/AI/BP_IA_Master.BP_IA_Master_C|GetBP_AC_HP _asbp_ia_master) _output_get)
          (Default|TakeDamage _asbp_ia_master _output_get)
          (Character|LaunchCharacter _asbp_ia_master (Math|Vector|MakeVector (.x (* (Math|Vector|Normalize (- (Transformation|GetActorLocation _asbp_ia_master) (Transformation|GetActorLocation))) 300)) (.y (* (Math|Vector|Normalize (- (Transformation|GetActorLocation _asbp_ia_master) (Transformation|GetActorLocation))) 300)) 5e+02) false false))
        (:CastFailed
          (bind _asbp_break_rocks (Utilities|Casting|CastToBP_BreakRocks _array_element))
          (Default|HPModification (Variables|/Game/Blueprints/BP_BreakRocks.BP_BreakRocks_C|GetBP_AC_HP _asbp_break_rocks) -1))))))

(fn ConstructionScript
  (|CallParentFunction))
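; BP_Damage is a short-lived floating damage number actor that displays an integer set through its setValue event.
; On BeginPlay, projectile movement launches it upward with one of two random sideways drifts, caps its max speed after a brief delay, then destroys the actor about a second after spawning.
; Each Tick rotates the text to face the top-down controller's camera, acting as a billboard.
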(event Custom|setValue
  (params (value :type Integer))
  (Rendering|Components|TextRender|SetText (Variables|Default|Getdamage) (Utilities|Text|ToText(Integer) value)))

(event EventBeginPlay
  (bind _projectilemovement (Variables|Default|GetProjectileMovement))
  (Components|Activation|SetActive _projectilemovement true false)
  (if (Math|Random|RandomBool)
    (Variables|/Script/Engine.MovementComponent|SetVelocity _projectilemovement "50.000000,-50.000000,800.000000")
    (else
      (Variables|/Script/Engine.MovementComponent|SetVelocity _projectilemovement "-50.000000,50.000000,800.000000")))
  (Utilities|FlowControl|Delay 0.2)
  (Variables|/Script/Engine.ProjectileMovementComponent|SetMaxSpeed (Variables|Default|GetProjectileMovement) 4e+02)
  (Utilities|FlowControl|Delay 0.8)
  (Actor|DestroyActor))

(event Collision|EventActorBeginOverlap
  (params (OtherActor :type Actor%20Object%20Reference)))

(event EventTick
  (params (DeltaSeconds :type Float%20%28single-precision%29))
  (Transformation|SetWorldRotation (Variables|Default|Getdamage) (Math|Rotator|FindLookatRotation (Transformation|GetWorldLocation (Variables|Default|Getdamage)) (Camera|GetCameraLocation (Variables|/Script/Engine.PlayerController|GetPlayerCameraManager (CallFunction|GetTopDownController)))) false false))

(fn ConstructionScript)
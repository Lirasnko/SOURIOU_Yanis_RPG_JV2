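; BP_Item is a world pickup actor that represents one item the player can collect.
; On BeginPlay it sets its static mesh from the mesh of its CurrentItem.
; Interact increments that item's count in the top-down controller's Inventory map, or adds it with a count of one, then destroys the actor.
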(event EventBeginPlay
  (|CallParentFunction)
  (Components|StaticMesh|SetStaticMesh (Variables|Default|GetStaticMesh) (Variables|/Game/Blueprints/Data/BP_PDA_Items.BP_PDA_Items_C|GetMesh (Variables|Default|GetCurrentItem))))

(event Collision|EventActorBeginOverlap
  (params (OtherActor :type Actor%20Object%20Reference))
  (|CallParentFunction OtherActor) ; This node is disabled and will not be called.\nDrag off pins to build functionality.
)

(event EventTick
  (params (DeltaSeconds :type Float%20%28single-precision%29))
  (|CallParentFunction DeltaSeconds) ; This node is disabled and will not be called.\nDrag off pins to build functionality.
)

(event EventInteract
  (bind _playercontroler (CallFunction|GetTopDownController))
  (bind _currentitem (Variables|Default|GetCurrentItem))
  (bind _inventory (Variables|/Game/TopDown/Blueprints/BP_TopDownController.BP_TopDownController_C|GetInventory _playercontroler))
  (bind (_value _returnvalue) (Utilities|Map|Find _inventory _currentitem))
  (if _returnvalue
    (Utilities|Map|Add _inventory _currentitem (+ _value 1))
    (else
      (Utilities|Map|Add _inventory _currentitem 1)))
  (Actor|DestroyActor))

(fn ConstructionScript
  (|CallParentFunction))
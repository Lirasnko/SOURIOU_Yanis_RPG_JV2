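; World pickup for an item data asset (CurrentItem), which sets its mesh and name label, plus rarity and element material colors for weapon items.
; When the top-down character enters TakeZone, it registers with the controller and shows its name and take prompt; leaving reverses both.
; While visible, both labels turn toward the camera each Tick.
; Take increments the item's count in the controller's Inventory map and destroys the actor.
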(event OnComponentBeginOverlap(TakeZone)
  (params (OverlappedComponent :type Primitive%20Component%20Object%20Reference) (OtherActor :type Actor%20Object%20Reference) (OtherComp :type Primitive%20Component%20Object%20Reference) (OtherBodyIndex :type Integer) (bFromSweep :type Boolean) (SweepResult :type Hit%20Result%20Structure%20%28by%20ref%29))
  (Utilities|Casting|CastToBP_TopDownCharacter OtherActor)
  (Default|SetTaking (CallFunction|GetTopDownController) self)
  (Rendering|SetVisibility (Variables|Default|GetObjectName) true false)
  (Rendering|SetVisibility (Variables|Default|GetTaking) true false))

(event OnComponentEndOverlap(TakeZone)
  (params (OverlappedComponent :type Primitive%20Component%20Object%20Reference) (OtherActor :type Actor%20Object%20Reference) (OtherComp :type Primitive%20Component%20Object%20Reference) (OtherBodyIndex :type Integer))
  (Utilities|Casting|CastToBP_TopDownCharacter OtherActor)
  (Default|RemoveTaking (CallFunction|GetTopDownController) self)
  (Rendering|SetVisibility (Variables|Default|GetObjectName) false false)
  (Rendering|SetVisibility (Variables|Default|GetTaking) false false))

(event Custom|Take
  (bind _playercontroler (CallFunction|GetTopDownController))
  (bind _currentitem (Variables|Default|GetCurrentItem))
  (bind _inventory (Variables|/Game/TopDown/Blueprints/BP_TopDownController.BP_TopDownController_C|GetInventory _playercontroler))
  (bind (_value _returnvalue) (Utilities|Map|Find _inventory _currentitem))
  (if _returnvalue
    (Utilities|Map|Add _inventory _currentitem (+ _value 1))
    (else
      (Utilities|Map|Add _inventory _currentitem 1)))
  (Actor|DestroyActor))

(event EventBeginPlay
  (Components|StaticMesh|SetStaticMesh (Variables|Default|GetObjectMesh) (Variables|/Game/Blueprints/Data/BP_PDA_Items.BP_PDA_Items_C|GetMesh (Variables|Default|GetCurrentItem)))
  (Rendering|Components|TextRender|SetText (Variables|Default|GetObjectName) (Variables|/Game/Blueprints/Data/BP_PDA_Items.BP_PDA_Items_C|GetName (Variables|Default|GetCurrentItem)))
  (Transformation|SetRelativeRotation (Variables|Default|GetObjectMesh) "0, 0, 0" false false)
  (bind _asbp_pda_weapons_items (Utilities|Casting|CastToBP_PDA_Weapons_Items (Variables|Default|GetCurrentItem)))
  (Default|SetRarityColor _asbp_pda_weapons_items)
  (Default|SetElementColor _asbp_pda_weapons_items)
  (Rendering|Material|SetColorParameterValueonMaterials (Variables|Default|GetObjectMesh) "ElementColor" (Math|Conversions|ToLinearColor(Color) (Variables|/Game/Blueprints/Data/BP_PDA_Weapons_Items.BP_PDA_Weapons_Items_C|GetElement_Color _asbp_pda_weapons_items)))
  (Rendering|Material|SetColorParameterValueonMaterials (Variables|Default|GetObjectMesh) "RarityColor" (Math|Conversions|ToLinearColor(Color) (Variables|/Game/Blueprints/Data/BP_PDA_Items.BP_PDA_Items_C|GetRarity_Color _asbp_pda_weapons_items))))

(event Collision|EventActorBeginOverlap
  (params (OtherActor :type Actor%20Object%20Reference)))

(event EventTick
  (params (DeltaSeconds :type Float%20%28single-precision%29))
  (bind _playercontroler (CallFunction|GetTopDownController))
  (bind _objectname (Variables|Default|GetObjectName))
  (bind _returnvalue (Transformation|GetWorldLocation _objectname))
  (bind _playercameramanager (Variables|/Script/Engine.PlayerController|GetPlayerCameraManager _playercontroler))
  (bind _returnvalue_2 (Camera|GetCameraLocation _playercameramanager))
  (bind _returnvalue_3 (Math|Rotator|FindLookatRotation _returnvalue _returnvalue_2))
  (if (Rendering|IsVisible (Variables|Default|GetObjectName))
    (Transformation|SetWorldRotation (Variables|Default|GetObjectName) _returnvalue_3 false false)
    (Transformation|SetWorldRotation (Variables|Default|GetTaking) _returnvalue_3 false false)))

(fn ConstructionScript)
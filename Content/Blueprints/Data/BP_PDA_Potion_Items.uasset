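; Potion item data asset that applies a Heal, Resistance, Strength or Speed effect to its user, scaled by a percentage Value.
; Use calls the parent, then heals from max HP or alters armor, attack bonus or walk speed, showing the buff's HUD icon and time.
; StopEffect hides those widgets and restores armor from a value cached on the asset, attack and speed from hardcoded defaults.
; No duration timing happens in these graphs.
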(fn Use
  (params (User :type BP%20Top%20Down%20Controller%20Object%20Reference))
  (bind _widgetgame (Variables|/Game/TopDown/Blueprints/BP_TopDownController.BP_TopDownController_C|GetWidgetGame User))
  (bind _widgetgame_2 (Variables|/Game/TopDown/Blueprints/BP_TopDownController.BP_TopDownController_C|GetWidgetGame User))
  (bind _widgetgame_3 (Variables|/Game/TopDown/Blueprints/BP_TopDownController.BP_TopDownController_C|GetWidgetGame User))
  (|CallParentFunction User)
  (switch Utilities|FlowControl|Switch|SwitchonE_Potion (Variables|Default|GetType)
    (:NewEnumerator0
      (Default|HPModification User (Math|Float|Truncate (* (Variables|/Game/TopDown/Blueprints/BP_TopDownController.BP_TopDownController_C|GetHPMax User) (/ (Math|Conversions|ToFloat(Integer) (Variables|Default|GetValue)) 1e+02)))))
    (:NewEnumerator1
      (Variables|Default|SetPlayerArmorPointBase (Variables|/Game/TopDown/Blueprints/BP_TopDownController.BP_TopDownController_C|GetArmorPoint User))
      (Variables|/Game/TopDown/Blueprints/BP_TopDownController.BP_TopDownController_C|SetArmorPoint User (Math|Float|Truncate (* (Variables|/Game/TopDown/Blueprints/BP_TopDownController.BP_TopDownController_C|GetArmorPoint User) (/ (Math|Conversions|ToFloat(Integer) (Variables|Default|GetValue)) 1e+02))))
      (Widget|SetVisibility (Variables|/Game/Widget/WBP_Game.WBP_Game_C|GetResistanceIcon _widgetgame_2) "Visible")
      (Widget|SetVisibility (Variables|/Game/Widget/WBP_Game.WBP_Game_C|GetResistanceTime _widgetgame_2) "Visible"))
    (:NewEnumerator5
      (Variables|/Game/TopDown/Blueprints/BP_TopDownController.BP_TopDownController_C|SetAttackBonus User (+ (Variables|Default|GetValue) 100))
      (Widget|SetVisibility (Variables|/Game/Widget/WBP_Game.WBP_Game_C|GetStrengthIcon _widgetgame_3) "Visible")
      (Widget|SetVisibility (Variables|/Game/Widget/WBP_Game.WBP_Game_C|GetStrengthTime _widgetgame_3) "Visible"))
    (:NewEnumerator6
      (Variables|/Script/Engine.CharacterMovementComponent|SetMaxWalkSpeed (Variables|/Script/Engine.Character|GetCharacterMovement (Variables|/Game/TopDown/Blueprints/BP_TopDownController.BP_TopDownController_C|GetPlayerCharacter User)) (* 6e+02 (+ (/ (Math|Conversions|ToFloat(Integer) (Variables|Default|GetValue)) 1e+02) 1.0)))
      (Widget|SetVisibility (Variables|/Game/Widget/WBP_Game.WBP_Game_C|GetSpeedIcon _widgetgame) "Visible")
      (Widget|SetVisibility (Variables|/Game/Widget/WBP_Game.WBP_Game_C|GetSpeedTime _widgetgame) "Visible"))))

(fn StopEffect
  (params (User :type BP%20Top%20Down%20Controller%20Object%20Reference) (Type :type E_Potion%20Enum :default "NewEnumerator0"))
  (bind _widgetgame (Variables|/Game/TopDown/Blueprints/BP_TopDownController.BP_TopDownController_C|GetWidgetGame User))
  (bind _widgetgame_2 (Variables|/Game/TopDown/Blueprints/BP_TopDownController.BP_TopDownController_C|GetWidgetGame User))
  (bind _widgetgame_3 (Variables|/Game/TopDown/Blueprints/BP_TopDownController.BP_TopDownController_C|GetWidgetGame User))
  (switch Utilities|FlowControl|Switch|SwitchonE_Potion Type
    (:NewEnumerator1
      (Widget|SetVisibility (Variables|/Game/Widget/WBP_Game.WBP_Game_C|GetResistanceIcon _widgetgame_2) "Hidden")
      (Widget|SetVisibility (Variables|/Game/Widget/WBP_Game.WBP_Game_C|GetResistanceTime _widgetgame_2) "Hidden")
      (Variables|/Game/TopDown/Blueprints/BP_TopDownController.BP_TopDownController_C|SetArmorPoint User (Variables|Default|GetPlayerArmorPointBase)))
    (:NewEnumerator5
      (Widget|SetVisibility (Variables|/Game/Widget/WBP_Game.WBP_Game_C|GetStrengthIcon _widgetgame) "Hidden")
      (Widget|SetVisibility (Variables|/Game/Widget/WBP_Game.WBP_Game_C|GetStrengthTime _widgetgame) "Hidden")
      (Variables|/Game/TopDown/Blueprints/BP_TopDownController.BP_TopDownController_C|SetAttackBonus User 100))
    (:NewEnumerator6
      (Widget|SetVisibility (Variables|/Game/Widget/WBP_Game.WBP_Game_C|GetSpeedIcon _widgetgame_3) "Hidden")
      (Widget|SetVisibility (Variables|/Game/Widget/WBP_Game.WBP_Game_C|GetSpeedTime _widgetgame_3) "Hidden")
      (Variables|/Script/Engine.CharacterMovementComponent|SetMaxWalkSpeed (Variables|/Script/Engine.Character|GetCharacterMovement (Variables|/Game/TopDown/Blueprints/BP_TopDownController.BP_TopDownController_C|GetPlayerCharacter User)) 6e+02))))
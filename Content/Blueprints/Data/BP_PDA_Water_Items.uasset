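; Water item data asset whose Use function refills the user's water from the selected inventory slot.
; After running the parent Use, it compares the slot's stored amount with the water the user is missing.
; A larger amount fills the user to WaterMax and writes the remainder back into the Slots map; otherwise the whole amount is added and the slot's value is set to zero.
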(fn Use
  (params (User :type BP%20Top%20Down%20Controller%20Object%20Reference))
  (bind _slots (Variables|/Game/TopDown/Blueprints/BP_TopDownController.BP_TopDownController_C|GetSlots User))
  (bind _selecteditemindex (Variables|/Game/TopDown/Blueprints/BP_TopDownController.BP_TopDownController_C|GetSelectedItemIndex User))
  (bind _watermax (Variables|/Game/TopDown/Blueprints/BP_TopDownController.BP_TopDownController_C|GetWaterMax User))
  (bind _water (Variables|/Game/TopDown/Blueprints/BP_TopDownController.BP_TopDownController_C|GetWater User))
  (bind (_key _value) (Utilities|Map|GetKeyValueByIndex _slots _selecteditemindex))
  (bind _returnvalue (- _watermax _water))
  (|CallParentFunction User)
  (bind _output_get (Variables|Default|SetWaterQuantity (- _value _returnvalue)))
  (if (> _value _returnvalue)
    (Default|WaterModification User _watermax)
    (Utilities|Map|Add _slots _key _output_get)
    (else
      (Default|WaterModification User (+ _water _value))
      (Utilities|Map|Add _slots _key 0))))
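; Item data asset Blueprint, named for weapons and items, that defines a rarity tint and a healing use action.
; Set_Sprite_Color maps Rarity to a fixed Color for each tier, from Common to Legendary, when IsRarityColor is enabled.
; Use does nothing at full HP; otherwise it runs the parent Use, then adds Durability to the user's HP, capped at HPMax.
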(event Custom|Set_Sprite_Color
  (if (Variables|Default|GetIsRarityColor)
    (switch Utilities|FlowControl|Switch|SwitchonE_Rarity (Variables|Default|GetRarity)
      (:NewEnumerator0
        (Variables|Default|SetColor (Math|Conversions|ToColor(LinearColor) (Math|Color|MakeColor 0.3 0.3 0.3))))
      (:NewEnumerator1
        (Variables|Default|SetColor (Math|Conversions|ToColor(LinearColor) (Math|Color|MakeColor 0.0 0.5 0.0))))
      (:NewEnumerator2
        (Variables|Default|SetColor (Math|Conversions|ToColor(LinearColor) (Math|Color|MakeColor 0.15 0.15 0.7))))
      (:NewEnumerator3
        (Variables|Default|SetColor (Math|Conversions|ToColor(LinearColor) (Math|Color|MakeColor 0.3 0.0 0.3))))
      (:NewEnumerator4
        (Variables|Default|SetColor (Math|Conversions|ToColor(LinearColor) (Math|Color|MakeColor 0.75 0.75 0.0)))))))

(fn Use
  (params (User :type BP%20Top%20Down%20Controller%20Object%20Reference))
  (bind _hpmax (Variables|/Game/TopDown/Blueprints/BP_TopDownController.BP_TopDownController_C|GetHPMax User))
  (if (not (== (Variables|/Game/TopDown/Blueprints/BP_TopDownController.BP_TopDownController_C|GetHP User) (Variables|/Game/TopDown/Blueprints/BP_TopDownController.BP_TopDownController_C|GetHPMax User)))
    (|CallParentFunction User)
    (if (> (+ (Variables|/Game/TopDown/Blueprints/BP_TopDownController.BP_TopDownController_C|GetHP User) (Variables|Default|GetDurability)) _hpmax)
      (Variables|/Game/TopDown/Blueprints/BP_TopDownController.BP_TopDownController_C|SetHP User _hpmax)
      (else
        (Variables|/Game/TopDown/Blueprints/BP_TopDownController.BP_TopDownController_C|SetHP User (+ (Variables|/Game/TopDown/Blueprints/BP_TopDownController.BP_TopDownController_C|GetHP User) (Variables|Default|GetDurability)))))))
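; Primary data asset Blueprint for items, carrying an element, a rarity and a display color for each.
; Two events, Set_Element_Color and Set_Rarity_Color, switch on the Element and Rarity enums and store a hard-coded sRGB-converted color in ElementColor and RarityColor.
; The Use function is a stub that only prints the display name of the user passed to it.
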(event Custom|Set_Element_Color
  (switch Utilities|FlowControl|Switch|SwitchonE_Element (Variables|Default|GetElement)
    (:NewEnumerator0
      (Variables|Default|SetElement_Color (Math|Conversions|ToColor(LinearColor) (Math|Color|MakeColor 0.95 0.1 0.1))))
    (:NewEnumerator1
      (Variables|Default|SetElement_Color (Math|Conversions|ToColor(LinearColor) (Math|Color|MakeColor 0.0 0.5 0.8))))
    (:NewEnumerator2
      (Variables|Default|SetElement_Color (Math|Conversions|ToColor(LinearColor) (Math|Color|MakeColor 1.0 1.0 0.0))))
    (:NewEnumerator3
      (Variables|Default|SetElement_Color (Math|Conversions|ToColor(LinearColor) (Math|Color|MakeColor 0.5 0.0 0.7))))
    (:NewEnumerator4
      (Variables|Default|SetElement_Color (Math|Conversions|ToColor(LinearColor) (Math|Color|MakeColor 0.1 1.0 0.9))))
    (:NewEnumerator5
      (Variables|Default|SetElement_Color (Math|Conversions|ToColor(LinearColor) (Math|Color|MakeColor 1.0 0.5 0.0))))
    (:NewEnumerator6
      (Variables|Default|SetElement_Color (Math|Conversions|ToColor(LinearColor) (Math|Color|MakeColor 0.3 0.3 0.3))))))

(event Custom|Set_Rarity_Color
  (switch Utilities|FlowControl|Switch|SwitchonE_Rarity (Variables|Default|GetRarity)
    (:NewEnumerator0
      (Variables|Default|SetRarity_Color (Math|Conversions|ToColor(LinearColor) (Math|Color|MakeColor 0.3 0.3 0.3))))
    (:NewEnumerator1
      (Variables|Default|SetRarity_Color (Math|Conversions|ToColor(LinearColor) (Math|Color|MakeColor 0.0 0.5 0.0))))
    (:NewEnumerator2
      (Variables|Default|SetRarity_Color (Math|Conversions|ToColor(LinearColor) (Math|Color|MakeColor 0.15 0.15 0.7))))
    (:NewEnumerator3
      (Variables|Default|SetRarity_Color (Math|Conversions|ToColor(LinearColor) (Math|Color|MakeColor 0.3 0.0 0.3))))
    (:NewEnumerator4
      (Variables|Default|SetRarity_Color (Math|Conversions|ToColor(LinearColor) (Math|Color|MakeColor 0.75 0.75 0.0))))))

(fn Use
  (params (User :type BP%20Top%20Down%20Controller%20Object%20Reference))
  (Development|PrintString 0 (Utilities|String|Append (Utilities|GetDisplayName User) "")))
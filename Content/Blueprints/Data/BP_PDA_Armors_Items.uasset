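; BP_PDA_Armors_Items is an item Blueprint, apparently a data asset for armor items, whose use restores HP to the user.
; Its Use override does nothing when the user's HP already equals HPMax.
; Otherwise it calls the parent Use, then adds the item's HP value to the user's HP, capped at HPMax.
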(fn Use
  (params (User :type BP%20Top%20Down%20Controller%20Object%20Reference))
  (bind _hpmax (Variables|/Game/TopDown/Blueprints/BP_TopDownController.BP_TopDownController_C|GetHPMax User))
  (if (not (== (Variables|/Game/TopDown/Blueprints/BP_TopDownController.BP_TopDownController_C|GetHP User) (Variables|/Game/TopDown/Blueprints/BP_TopDownController.BP_TopDownController_C|GetHPMax User)))
    (|CallParentFunction User)
    (if (> (+ (Variables|/Game/TopDown/Blueprints/BP_TopDownController.BP_TopDownController_C|GetHP User) (Variables|Default|GetHP)) _hpmax)
      (Variables|/Game/TopDown/Blueprints/BP_TopDownController.BP_TopDownController_C|SetHP User _hpmax)
      (else
        (Variables|/Game/TopDown/Blueprints/BP_TopDownController.BP_TopDownController_C|SetHP User (+ (Variables|/Game/TopDown/Blueprints/BP_TopDownController.BP_TopDownController_C|GetHP User) (Variables|Default|GetHP)))))))
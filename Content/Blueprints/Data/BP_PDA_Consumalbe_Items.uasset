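; Consumable item data asset that restores the user's Food or Water when used.
; Use calls the parent implementation, then switches on Type to add Value to the matching stat, capped at its maximum.
; When Water reaches or exceeds its cap, the amount used is subtracted from the asset's own Value, leaving the remainder; other branches leave Value unchanged.
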(fn Use
  (params (User :type BP%20Top%20Down%20Controller%20Object%20Reference))
  (bind _watermax (Variables|/Game/TopDown/Blueprints/BP_TopDownController.BP_TopDownController_C|GetWaterMax User))
  (bind _foodmax (Variables|/Game/TopDown/Blueprints/BP_TopDownController.BP_TopDownController_C|GetFoodMax User))
  (|CallParentFunction User)
  (switch Utilities|FlowControl|Switch|SwitchonE_Food (Variables|Default|GetType)
    (:NewEnumerator0
      (if (>= (+ (Variables|/Game/TopDown/Blueprints/BP_TopDownController.BP_TopDownController_C|GetFood User) (Variables|Default|GetValue)) _foodmax)
        (Variables|/Game/TopDown/Blueprints/BP_TopDownController.BP_TopDownController_C|SetFood User _foodmax)
        (else
          (Variables|/Game/TopDown/Blueprints/BP_TopDownController.BP_TopDownController_C|SetFood User (+ (Variables|/Game/TopDown/Blueprints/BP_TopDownController.BP_TopDownController_C|GetFood User) (Variables|Default|GetValue))))))
    (:NewEnumerator1
      (if (>= (+ (Variables|/Game/TopDown/Blueprints/BP_TopDownController.BP_TopDownController_C|GetWater User) (Variables|Default|GetValue)) _watermax)
        (Variables|Default|SetValue (- (Variables|Default|GetValue) (- _watermax (Variables|/Game/TopDown/Blueprints/BP_TopDownController.BP_TopDownController_C|GetWater User))))
        (Variables|/Game/TopDown/Blueprints/BP_TopDownController.BP_TopDownController_C|SetWater User _watermax)
        (else
          (Variables|/Game/TopDown/Blueprints/BP_TopDownController.BP_TopDownController_C|SetWater User (+ (Variables|/Game/TopDown/Blueprints/BP_TopDownController.BP_TopDownController_C|GetWater User) (Variables|Default|GetValue))))))))
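; BP_AC_HP is a health component that stores HP for the player or other actors and handles their death.
; HPModification applies a signed change clamped between zero and HPMax, pushing the HP percent to the game widget for the player while they survive.
; At zero, non-player actors are destroyed.
; Player death refills the controller's HP, Food and Water, flags InHub, calls SetGameInstance and loads the hub level.
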(event EventBeginPlay)

(event EventTick
  (params (DeltaSeconds :type Float%20%28single-precision%29)))

(fn HPModification
  (params (Quantity :type Integer) (isPlayer :type Boolean))
  (bind _hpmax (Variables|Default|GetHPMax))
  (if (> Quantity 0)
    (if (> (- _hpmax (Variables|Default|GetHP)) Quantity)
      (Variables|Default|SetHP (+ (Variables|Default|GetHP) Quantity))
      (else
        (Variables|Default|SetHP _hpmax)))
    (if isPlayer :!label _label
      (Variables|/Game/Widget/WBP_Game.WBP_Game_C|SetPlayerHPPercent (Variables|/Game/TopDown/Blueprints/BP_TopDownController.BP_TopDownController_C|GetWidgetGame (CallFunction|GetTopDownController)) (/ (Math|Conversions|ToFloat(Integer) (Variables|Default|GetHP)) (Math|Conversions|ToFloat(Integer) (Variables|Default|GetHPMax)))))
    (elif (> (Variables|Default|GetHP) (* Quantity -1))
      (Variables|Default|SetHP (+ (Variables|Default|GetHP) Quantity))
      (goto _label)
      (else
        (Variables|Default|SetHP 0)
        (if isPlayer
          (CallFunction|PlayerDeath)
          (else
            (CallFunction|Death)))))))

(fn Death
  (Actor|DestroyActor (Variables|Default|GetActor)))

(fn PlayerDeath
  (bind _playercontroler (CallFunction|GetTopDownController))
  (bind _bp_ac_hp (Variables|/Game/TopDown/Blueprints/BP_TopDownController.BP_TopDownController_C|GetBP_AC_HP _playercontroler))
  (Variables|BP_AC_HP_C|SetHP _bp_ac_hp (Variables|BP_AC_HP_C|GetHPMax _bp_ac_hp))
  (Variables|/Game/TopDown/Blueprints/BP_TopDownController.BP_TopDownController_C|SetFood _playercontroler (Variables|/Game/TopDown/Blueprints/BP_TopDownController.BP_TopDownController_C|GetFoodMax _playercontroler))
  (Variables|/Game/TopDown/Blueprints/BP_TopDownController.BP_TopDownController_C|SetWater _playercontroler (Variables|/Game/TopDown/Blueprints/BP_TopDownController.BP_TopDownController_C|GetWaterMax _playercontroler))
  (Variables|/Game/TopDown/Blueprints/BP_TopDownController.BP_TopDownController_C|SetinHub _playercontroler true)
  (Default|SetGameInstance _playercontroler)
  (Game|OpenLevel(byObjectReference) "/Game/Level/Lvl_Hub.Lvl_Hub"))
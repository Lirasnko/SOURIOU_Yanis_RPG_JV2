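; BP_Exit is an interactable exit that sends the player back to the hub level.
; On Interact, it flags the TopDown controller as in the hub and refills HP, food and water to their maximums.
; It then calls SetGameInstance on that controller and opens Lvl_Hub by object reference.
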(event EventBeginPlay
  (|CallParentFunction) ; This node is disabled and will not be called.\nDrag off pins to build functionality.
)

(event Collision|EventActorBeginOverlap
  (params (OtherActor :type Actor%20Object%20Reference))
  (|CallParentFunction OtherActor) ; This node is disabled and will not be called.\nDrag off pins to build functionality.
)

(event EventTick
  (params (DeltaSeconds :type Float%20%28single-precision%29))
  (|CallParentFunction DeltaSeconds) ; This node is disabled and will not be called.\nDrag off pins to build functionality.
)

(event EventInteract
  (bind _playercontroler (CallFunction|GetTopDownController))
  (bind _bp_ac_hp (Variables|/Game/TopDown/Blueprints/BP_TopDownController.BP_TopDownController_C|GetBP_AC_HP _playercontroler))
  (Variables|/Game/TopDown/Blueprints/BP_TopDownController.BP_TopDownController_C|SetinHub _playercontroler true)
  (Variables|/Game/Blueprints/Component/BP_AC_HP.BP_AC_HP_C|SetHP _bp_ac_hp (Variables|/Game/Blueprints/Component/BP_AC_HP.BP_AC_HP_C|GetHPMax _bp_ac_hp))
  (Variables|/Game/TopDown/Blueprints/BP_TopDownController.BP_TopDownController_C|SetFood _playercontroler (Variables|/Game/TopDown/Blueprints/BP_TopDownController.BP_TopDownController_C|GetFoodMax _playercontroler))
  (Variables|/Game/TopDown/Blueprints/BP_TopDownController.BP_TopDownController_C|SetWater _playercontroler (Variables|/Game/TopDown/Blueprints/BP_TopDownController.BP_TopDownController_C|GetWaterMax _playercontroler))
  (Default|SetGameInstance (CallFunction|GetTopDownController))
  (Game|OpenLevel(byObjectReference) "/Game/Level/Lvl_Hub.Lvl_Hub"))

(fn ConstructionScript
  (|CallParentFunction))
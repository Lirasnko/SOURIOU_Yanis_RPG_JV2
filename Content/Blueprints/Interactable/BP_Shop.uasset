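; BP_Shop is an interactable shop that registers with the top-down controller and shows a text prompt while the player character overlaps its trigger.
; Interacting while Open is true clears that flag, swaps the game HUD for the shop widget, blends the camera to the shop and timeline-lerps the player to a shop-relative spot.
; Otherwise, it closes open widgets and ResetPosition returns camera and player.
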(event OnComponentBeginOverlap(Player_Position)
  (params (OverlappedComponent :type Primitive%20Component%20Object%20Reference) (OtherActor :type Actor%20Object%20Reference) (OtherComp :type Primitive%20Component%20Object%20Reference) (OtherBodyIndex :type Integer) (bFromSweep :type Boolean) (SweepResult :type Hit%20Result%20Structure%20%28by%20ref%29))
  (Utilities|Casting|CastToBP_TopDownCharacter OtherActor)
  (Default|SetInteractable (CallFunction|GetTopDownController) self)
  (Rendering|SetVisibility (Variables|Default|GetTextRender) true false))

(event OnComponentEndOverlap(Player_Position)
  (params (OverlappedComponent :type Primitive%20Component%20Object%20Reference) (OtherActor :type Actor%20Object%20Reference) (OtherComp :type Primitive%20Component%20Object%20Reference) (OtherBodyIndex :type Integer))
  (Utilities|Casting|CastToBP_TopDownCharacter OtherActor)
  (Default|RemoveInteractable (CallFunction|GetTopDownController) self)
  (Rendering|SetVisibility (Variables|Default|GetTextRender) false false))

(event Custom|ResetPosition
  (bind _playercontroler (CallFunction|GetTopDownController))
  (Game|Player|SetViewTargetwithBlend _playercontroler (Pawn|GetControlledPawn _playercontroler) 0.5 "VTBlend_Linear" 0.0 false)
  (bind _newtrack_0 (Timeline|Timeline_0 Play)
    (:Update
      (Transformation|SetActorLocationAndRotation (Game|Player|GetPlayerPawn 0) (Math|Vector|Lerp(Vector) (+ (Transformation|GetActorLocation) (Math|Vector|RotateVector (Variables|/Script/Engine.SceneComponent|GetRelativeLocation (Variables|Default|GetPlayer_Position)) (Transformation|GetActorRotation))) (Variables|Default|GetPlayerPosition) _newtrack_0)))))

(event EventBeginPlay
  (|CallParentFunction) ; This node is disabled and will not be called.\nDrag off pins to build functionality.
)

(event Collision|EventActorBeginOverlap
  (params (OtherActor :type Actor%20Object%20Reference))
  (|CallParentFunction OtherActor) ; This node is disabled and will not be called.\nDrag off pins to build functionality.
)

(event EventTick
  (params (DeltaSeconds :type Float%20%28single-precision%29))
  (|CallParentFunction DeltaSeconds) ; This node is disabled and will not be called.\nDrag off pins to build functionality.
)

(event EventInteract
  (bind _playercontroler (CallFunction|GetTopDownController))
  (bind _widgetgame (Variables|/Game/TopDown/Blueprints/BP_TopDownController.BP_TopDownController_C|GetWidgetGame _playercontroler))
  (bind _widgetshop (Variables|/Game/TopDown/Blueprints/BP_TopDownController.BP_TopDownController_C|GetWidgetShop _playercontroler))
  (|CallParentFunction)
  (if (Variables|Default|Getopen)
    (Variables|Default|Setopen false)
    (Widget|SetVisibility _widgetgame "Hidden")
    (for _array_element (Variables|/Game/Widget/WBP_Game.WBP_Game_C|GetItems _widgetgame)
      (Widget|SetVisibility _array_element "Hidden"))
    (Default|Open _widgetshop)
    (Widget|SetVisibility _widgetshop "Visible")
    (Game|Player|SetViewTargetwithBlend (CallFunction|GetTopDownController) self 0.5 "VTBlend_Linear" 0.0 false)
    (bind _output_get (Variables|Default|SetPlayerPosition (Transformation|GetActorLocation (Game|Player|GetPlayerPawn 0))))
    (bind _newtrack_0 (Timeline|Timeline Play)
      (:Update
        (Transformation|SetActorLocationAndRotation (Game|Player|GetPlayerPawn 0) (Math|Vector|Lerp(Vector) _output_get (+ (Transformation|GetActorLocation) (Math|Vector|RotateVector (Variables|/Script/Engine.SceneComponent|GetRelativeLocation (Variables|Default|GetPlayer_Position)) (Transformation|GetActorRotation))) _newtrack_0))
        (Rendering|SetVisibility (Variables|Default|GetTextRender) false false)))
    (else
      (Default|CloseOpenWidgets _playercontroler)
      (CallFunction|ResetPosition)
      (Rendering|SetVisibility (Variables|Default|GetTextRender) true false))))

(fn ConstructionScript
  (|CallParentFunction))
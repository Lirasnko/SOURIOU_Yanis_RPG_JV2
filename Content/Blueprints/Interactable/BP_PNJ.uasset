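; Interactable NPC actor that shows its Name on a text render component and moves the player into a conversation spot when used.
; Interact alternates through a FlipFlop: the first call flags the top-down controller as interacting, saves the player's transform and timeline-lerps the pawn to an offset relative to the NPC.
; The next call lerps it back and clears the flag.
; Camera view-target blending nodes exist but are unwired.
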(event EventBeginPlay
  (|CallParentFunction)
  (Rendering|Components|TextRender|SetText (Variables|Default|GetTextRender) (Variables|Default|GetName)))

(event Collision|EventActorBeginOverlap
  (params (OtherActor :type Actor%20Object%20Reference))
  (|CallParentFunction OtherActor) ; This node is disabled and will not be called.\nDrag off pins to build functionality.
)

(event EventTick
  (params (DeltaSeconds :type Float%20%28single-precision%29))
  (|CallParentFunction DeltaSeconds) ; This node is disabled and will not be called.\nDrag off pins to build functionality.
)

(event EventInteract
  (Utilities|FlowControl|FlipFlop
    (:A
      (Variables|/Game/TopDown/Blueprints/BP_TopDownController.BP_TopDownController_C|SetisInteracting (CallFunction|GetTopDownController) true)
      (bind _output_get (Variables|Default|SetplayerRotation (Transformation|GetActorRotation (Game|Player|GetPlayerPawn 0))))
      (bind _output_get_2 (Variables|Default|SetplayerPosition (Transformation|GetActorLocation (Game|Player|GetPlayerPawn 0))))
      (bind _newtrack_0 (Timeline|Timeline Play)
        (:Update
          (Transformation|SetActorLocationAndRotation (Game|Player|GetPlayerPawn 0) (Math|Vector|Lerp(Vector) _output_get_2 (+ (Transformation|GetActorLocation) (Math|Vector|RotateVector (Variables|/Script/Engine.SceneComponent|GetRelativeLocation (Variables|Default|GetPlayer_Position)) (Transformation|GetActorRotation))) _newtrack_0) (Math|Rotator|Lerp(Rotator) _output_get (Math|Rotator|CombineRotators (Transformation|GetActorRotation) "0.000000,10.000000,0.000000") _newtrack_0 true)))))
    (:B
      (bind _newtrack_0_2 (Timeline|Timeline_0 Play)
        (:Update
          (Transformation|SetActorLocationAndRotation (Game|Player|GetPlayerPawn 0) (Math|Vector|Lerp(Vector) (+ (Transformation|GetActorLocation) (Math|Vector|RotateVector (Variables|/Script/Engine.SceneComponent|GetRelativeLocation (Variables|Default|GetPlayer_Position)) (Transformation|GetActorRotation))) (Variables|Default|GetplayerPosition) _newtrack_0_2) (Math|Rotator|Lerp(Rotator) (Math|Rotator|CombineRotators (Transformation|GetActorRotation) "0.000000,10.000000,0.000000") (Variables|Default|GetplayerRotation) _newtrack_0_2 true))
          (Variables|/Game/TopDown/Blueprints/BP_TopDownController.BP_TopDownController_C|SetisInteracting (CallFunction|GetTopDownController) false))))))

(fn ConstructionScript
  (|CallParentFunction))
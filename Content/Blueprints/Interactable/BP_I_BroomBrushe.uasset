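; BP_I_BroomBrushe is an interactable pickup actor for a broom brush item.
; On Interact, it adds one DA_I_BroomBrush data asset to the top-down controller's inventory and destroys itself.
; It has no other active logic; its construction script only calls the parent.
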(event EventBeginPlay
  (|CallParentFunction) ; This node is disabled and will not be called.\nDrag off pins to build functionality.
)

(event Collision|EventActorBeginOverlap
  (params (OtherActor :type Actor%20Object%20Reference))
  (|CallParentFunction OtherActor) ; This node is disabled and will not be called.\nDrag off pins to build functionality.
)

(event EventTick
  (params (DeltaSeconds :type Float%20%28single-precision%29))
  (|CallParentFunction DeltaSeconds) ; This node is disabled and will not be called.\nDrag off pins to build functionality.
)

(event EventInteract
  (Utilities|Map|Add (Variables|/Game/TopDown/Blueprints/BP_TopDownController.BP_TopDownController_C|GetInventory (CallFunction|GetTopDownController)) "/Game/Data/Items/DA_I_BroomBrush.DA_I_BroomBrush" 1)
  (Actor|DestroyActor))

(fn ConstructionScript
  (|CallParentFunction))
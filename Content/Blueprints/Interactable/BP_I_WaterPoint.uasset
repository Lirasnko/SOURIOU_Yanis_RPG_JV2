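; Interactable water point that refills the three water item types held by the player's top-down controller.
; On Interact, Add_Water runs per type on the Slots map, re-adding an entry with its key's Value and printing it, while Inventory entries are set to fixed per-type amounts.
; Add_Water's index counter advances only on a key match, so its by-index lookup does not track the item's actual map position.
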(event Custom|Add_Water
  (params (Water :type BP%20PDA%20Water%20Items%20Object%20Reference) (Items :type Map%20of%20BP%20PDA%20Items%20Object%20References%20to%20Integers))
  (Variables|Default|Setindex 0)
  (bind _keypin (Utilities|Map|ForEachLoop(Map) Items)
    (:then
      (if (== _keypin Water)
        (Variables|Default|SetindexOf (Variables|Default|Getindex))
        (Variables|Default|Setindex (+ (Variables|Default|Getindex) 1))))
    (:CompletedPin
      (if (.ReturnValue (Utilities|Map|Find Items Water))
        (Utilities|Map|Add Items (.Key (Utilities|Map|GetKeyValueByIndex Items (Variables|Default|GetindexOf))) (Variables|/Game/Blueprints/Data/BP_PDA_Items.BP_PDA_Items_C|GetValue (.Key (Utilities|Map|GetKeyValueByIndex Items (Variables|Default|GetindexOf)))))
        (Development|PrintString (Utilities|String|ToString(Integer) (Variables|/Game/Blueprints/Data/BP_PDA_Items.BP_PDA_Items_C|GetValue (.Key (Utilities|Map|GetKeyValueByIndex Items (Variables|Default|GetindexOf))))))))))

(event EventBeginPlay
  (|CallParentFunction) ; This node is disabled and will not be called.\nDrag off pins to build functionality.
)

(event Collision|EventActorBeginOverlap
  (params (OtherActor :type Actor%20Object%20Reference))
  (|CallParentFunction OtherActor) ; This node is disabled and will not be called.\nDrag off pins to build functionality.
)

(event EventTick
  (params (DeltaSeconds :type Float%20%28single-precision%29))
  (|CallParentFunction DeltaSeconds) ; This node is disabled and will not be called.\nDrag off pins to build functionality.
)

(event EventInteract
  (bind _playercontroler (CallFunction|GetTopDownController))
  (bind _slots (Variables|/Game/TopDown/Blueprints/BP_TopDownController.BP_TopDownController_C|GetSlots _playercontroler))
  (bind _inventory (Variables|/Game/TopDown/Blueprints/BP_TopDownController.BP_TopDownController_C|GetInventory _playercontroler))
  (CallFunction|AddWater "/Game/Data/Items/DA_IWa_Water_01.DA_IWa_Water_01" _slots)
  (CallFunction|AddWater "/Game/Data/Items/DA_IWa_Water_02.DA_IWa_Water_02" _slots)
  (CallFunction|AddWater "/Game/Data/Items/DA_IWa_Water_03.DA_IWa_Water_03" _slots)
  (if (.ReturnValue (Utilities|Map|Find _inventory "/Game/Data/Items/DA_IWa_Water_01.DA_IWa_Water_01"))
    (Utilities|Map|Add _inventory "/Game/Data/Items/DA_IWa_Water_01.DA_IWa_Water_01" 100))
  (if (.ReturnValue (Utilities|Map|Find _inventory "/Game/Data/Items/DA_IWa_Water_02.DA_IWa_Water_02"))
    (Utilities|Map|Add _inventory "/Game/Data/Items/DA_IWa_Water_02.DA_IWa_Water_02" 400))
  (if (.ReturnValue (Utilities|Map|Find _inventory "/Game/Data/Items/DA_IWa_Water_03.DA_IWa_Water_03"))
    (Utilities|Map|Add _inventory "/Game/Data/Items/DA_IWa_Water_03.DA_IWa_Water_03" 1000)))

(fn ConstructionScript
  (|CallParentFunction))
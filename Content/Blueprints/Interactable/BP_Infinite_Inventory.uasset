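; BP_Infinite_Inventory is an interactable that gives access to the infinite inventory screen.
; Interact runs the parent logic, then checks Open: if true, it clears the flag, hides the game widget, and opens and shows the infinite inventory widget through the top-down controller.
; Otherwise it tells the controller to close any open widgets.
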(event EventBeginPlay
  (|CallParentFunction) ; This node is disabled and will not be called.\nDrag off pins to build functionality.
)

(event Collision|EventActorBeginOverlap
  (params (OtherActor :type Actor%20Object%20Reference))
  (|CallParentFunction OtherActor) ; This node is disabled and will not be called.\nDrag off pins to build functionality.
)

(event EventTick
  (params (DeltaSeconds :type Float%20%28single-precision%29))
  (|CallParentFunction DeltaSeconds) ; This node is disabled and will not be called.\nDrag off pins to build functionality.
)

(event EventInteract
  (bind _playercontroler (CallFunction|GetTopDownController))
  (bind _widgetinfiniteinventory (Variables|/Game/TopDown/Blueprints/BP_TopDownController.BP_TopDownController_C|GetWidgetInfiniteInventory _playercontroler))
  (|CallParentFunction)
  (if (Variables|Default|Getopen)
    (Variables|Default|Setopen false)
    (Widget|SetVisibility (Variables|/Game/TopDown/Blueprints/BP_TopDownController.BP_TopDownController_C|GetWidgetGame _playercontroler) "Hidden")
    (Default|Open _widgetinfiniteinventory)
    (Widget|SetVisibility _widgetinfiniteinventory "Visible")
    (else
      (Default|CloseOpenWidgets _playercontroler))))

(fn ConstructionScript
  (|CallParentFunction))
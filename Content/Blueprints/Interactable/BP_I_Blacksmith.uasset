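; Interactable blacksmith that trades the broom brush item for money.
; On Interact it looks for the DA_I_BroomBrush data asset in the top-down controller's Inventory, then falls back to its Slots.
; If found, it removes the item from that container and adds a fixed reward to the controller's Money; otherwise nothing happens.
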(event EventBeginPlay
  (|CallParentFunction) ; This node is disabled and will not be called.\nDrag off pins to build functionality.
)

(event Collision|EventActorBeginOverlap
  (params (OtherActor :type Actor%20Object%20Reference))
  (|CallParentFunction OtherActor) ; This node is disabled and will not be called.\nDrag off pins to build functionality.
)

(event EventTick
  (params (DeltaSeconds :type Float%20%28single-precision%29))
  (|CallParentFunction DeltaSeconds) ; This node is disabled and will not be called.\nDrag off pins to build functionality.
)

(event EventInteract
  (bind _playercontroler (CallFunction|GetTopDownController))
  (bind _inventory (Variables|/Game/TopDown/Blueprints/BP_TopDownController.BP_TopDownController_C|GetInventory _playercontroler))
  (bind _slots (Variables|/Game/TopDown/Blueprints/BP_TopDownController.BP_TopDownController_C|GetSlots _playercontroler))
  (if (.ReturnValue (Utilities|Map|Find _inventory "/Game/Data/Items/DA_I_BroomBrush.DA_I_BroomBrush"))
    (Utilities|Map|Remove _inventory "/Game/Data/Items/DA_I_BroomBrush.DA_I_BroomBrush")
    (Variables|/Game/TopDown/Blueprints/BP_TopDownController.BP_TopDownController_C|SetMoney _playercontroler (+ (Variables|/Game/TopDown/Blueprints/BP_TopDownController.BP_TopDownController_C|GetMoney _playercontroler) 1000) :!label _label)
    (elif (.ReturnValue (Utilities|Map|Find _slots "/Game/Data/Items/DA_I_BroomBrush.DA_I_BroomBrush"))
      (Utilities|Map|Remove _slots "/Game/Data/Items/DA_I_BroomBrush.DA_I_BroomBrush")
      (goto _label))))

(fn ConstructionScript
  (|CallParentFunction))
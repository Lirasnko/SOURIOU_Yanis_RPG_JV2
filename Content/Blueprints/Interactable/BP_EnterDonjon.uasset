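; Interactable dungeon entrance that takes the player out of the hub and into the first donjon room level.
; On BeginPlay it copies the Donjon array from the top-down game instance when that array is not empty.
; On Interact it clears the controller's InHub flag, calls SetGameInstance on the controller, then opens Lvl_DonjonRoom_01 directly, independent of the copied array.
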(event EventBeginPlay
  (|CallParentFunction)
  (bind _asbp_game_instance_top_down (Utilities|Casting|CastToBP_GameInstance_TopDown (Game|GetGameInstance)))
  (if (> (Utilities|Array|Length (Variables|/Game/Blueprints/BP_GameInstance_TopDown.BP_GameInstance_TopDown_C|GetDonjon _asbp_game_instance_top_down)) 0)
    (Variables|Default|SetDonjon (Variables|/Game/Blueprints/BP_GameInstance_TopDown.BP_GameInstance_TopDown_C|GetDonjon _asbp_game_instance_top_down))))

(event Collision|EventActorBeginOverlap
  (params (OtherActor :type Actor%20Object%20Reference))
  (|CallParentFunction OtherActor) ; This node is disabled and will not be called.\nDrag off pins to build functionality.
)

(event EventTick
  (params (DeltaSeconds :type Float%20%28single-precision%29))
  (|CallParentFunction DeltaSeconds) ; This node is disabled and will not be called.\nDrag off pins to build functionality.
)

(event EventInteract
  (Variables|/Game/TopDown/Blueprints/BP_TopDownController.BP_TopDownController_C|SetinHub (CallFunction|GetTopDownController) false)
  (Default|SetGameInstance (CallFunction|GetTopDownController))
  (Game|OpenLevel(byObjectReference) "/Game/Level/Lvl_DonjonRoom_01.Lvl_DonjonRoom_01"))

(fn ConstructionScript
  (|CallParentFunction))
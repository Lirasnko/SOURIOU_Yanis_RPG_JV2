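; Interactable actor that toggles the infinite inventory screen in the top-down game.
; Interact alternates through a FlipFlop between opening and closing the inventory widget held by the game widget on the top-down controller.
; Opening clears the controller's InGame flag, sets IsInteracting, hides the game UI and shows each item widget; closing reverses those states without a matching close call.
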(event EventBeginPlay
  (|CallParentFunction) ; This node is disabled and will not be called.\nDrag off pins to build functionality.
)

(event Collision|EventActorBeginOverlap
  (params (OtherActor :type Actor%20Object%20Reference))
  (|CallParentFunction OtherActor) ; This node is disabled and will not be called.\nDrag off pins to build functionality.
)

(event EventTick
  (params (DeltaSeconds :type Float%20%28single-precision%29))
  (|CallParentFunction DeltaSeconds) ; This node is disabled and will not be called.\nDrag off pins to build functionality.
)

(event EventInteract
  (bind _playercontroler (CallFunction|GetTopDownController))
  (bind _widgetgame (Variables|/Game/TopDown/Blueprints/BP_TopDownController.BP_TopDownController_C|GetWidgetGame _playercontroler))
  (bind _widget_infiniteinventory (Variables|/Game/Widget/WBP_Game.WBP_Game_C|GetWidget_InfiniteInventory _widgetgame))
  (bind _items (Variables|/Game/Widget/WBP_InfiniteInventory.WBP_InfiniteInventory_C|GetItems _widget_infiniteinventory))
  ;[0.15 0.15 0.15 0.5] Open and close infinite inventory
  (Utilities|FlowControl|FlipFlop
    (:A
      (Variables|/Game/TopDown/Blueprints/BP_TopDownController.BP_TopDownController_C|SetinGame _playercontroler false)
      (Default|Open _widget_infiniteinventory)
      (Widget|SetVisibility _widget_infiniteinventory "Visible")
      (Variables|/Game/TopDown/Blueprints/BP_TopDownController.BP_TopDownController_C|SetisInteracting _playercontroler true)
      (Default|SetVisibilityUI _widgetgame "Hidden")
      (for _array_element _items
        (Widget|SetVisibility _array_element "Visible")))
    (:B
      (Variables|/Game/TopDown/Blueprints/BP_TopDownController.BP_TopDownController_C|SetinGame _playercontroler true)
      (Widget|SetVisibility _widget_infiniteinventory "Hidden")
      (Variables|/Game/TopDown/Blueprints/BP_TopDownController.BP_TopDownController_C|SetisInteracting _playercontroler false)
      (Default|SetVisibilityUI _widgetgame "Visible")
      (for _array_element_2 _items
        (Widget|SetVisibility _array_element_2 "Hidden")))))

(fn ConstructionScript
  (|CallParentFunction))
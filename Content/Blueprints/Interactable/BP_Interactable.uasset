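; BP_Interactable is an interactable actor with an empty Interact event, apparently a base for specific interactables.
; When a BP_TopDownCharacter enters or leaves its sphere, it registers or removes itself with the top-down controller and shows or hides its text prompt.
; While the text is visible, Tick rotates it to face the player camera.
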(event OnComponentBeginOverlap(Sphere)
  (params (OverlappedComponent :type Primitive%20Component%20Object%20Reference) (OtherActor :type Actor%20Object%20Reference) (OtherComp :type Primitive%20Component%20Object%20Reference) (OtherBodyIndex :type Integer) (bFromSweep :type Boolean) (SweepResult :type Hit%20Result%20Structure%20%28by%20ref%29))
  (Utilities|Casting|CastToBP_TopDownCharacter OtherActor)
  (Default|SetInteractable (CallFunction|GetTopDownController) self)
  (Rendering|SetVisibility (Variables|Default|GetTextRender) true false))

(event OnComponentEndOverlap(Sphere)
  (params (OverlappedComponent :type Primitive%20Component%20Object%20Reference) (OtherActor :type Actor%20Object%20Reference) (OtherComp :type Primitive%20Component%20Object%20Reference) (OtherBodyIndex :type Integer))
  (Utilities|Casting|CastToBP_TopDownCharacter OtherActor)
  (Default|RemoveInteractable (CallFunction|GetTopDownController) self)
  (Rendering|SetVisibility (Variables|Default|GetTextRender) false false))

(event Custom|Interact)

(event EventBeginPlay)

(event Collision|EventActorBeginOverlap
  (params (OtherActor :type Actor%20Object%20Reference)))

(event EventTick
  (params (DeltaSeconds :type Float%20%28single-precision%29))
  (if (Rendering|IsVisible (Variables|Default|GetTextRender))
    (Transformation|SetWorldRotation (Variables|Default|GetTextRender) (Math|Rotator|FindLookatRotation (Transformation|GetWorldLocation (Variables|Default|GetTextRender)) (Camera|GetCameraLocation (Variables|/Script/Engine.PlayerController|GetPlayerCameraManager (CallFunction|GetTopDownController)))) false false)))

(fn ConstructionScript)